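; Spawner actor that repeatedly spawns a configurable actor class at random points inside its box.
; Activation, triggered on BeginPlay when flagged to start active or through the Activate event, runs only once via an active flag.
; After a start delay it spawns immediately, then keeps spawning on a looping timer set by the cooldown.
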(event `spawn timer`
  (bind _box (`self.Box`))
  (`|SpawnActorFromClass` (`self.actor to spawn`) (`KismetMathLibrary.MakeTransform` (`KismetMathLibrary.RandomPointInBoundingBox` (`SceneComponent.K2_GetComponentLocation` _box) (`BoxComponent.BoxExtent` _box))) "Undefined" "OverrideRootScale"))

(event `activate`
  (if (not (`self.isactive`))
    (set `self.isactive` true)
    (`KismetSystemLibrary.Delay` (`self.start time`))
    (`KismetSystemLibrary.K2_SetTimerDelegate` (delegate `spawn timer`) (`self.spawn cooldown`) true)
    (`self.spawn timer`)))

(event `self.ReceiveBeginPlay`
  (if (`self.startactivated`)
    (`self.activate`)))

(fn `UserConstructionScript`)